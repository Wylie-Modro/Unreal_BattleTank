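; Player-controllable tank Blueprint that wires input to aiming, track-based movement, firing and camera components.
; On BeginPlay it hands barrel and turret to TankAiming, both tracks to TankMovement, and itself to the health bar widget.
; Input drives per-track throttle or directional movement intents, fires through TankAiming on right mouse release, and rotates a gimbal and spring arm for camera look.
; SwitchCamera toggles the first- and third-person cameras.
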(event EventBeginPlay
  (Class|TankAimingComponent|Initialise (Variables|Default|GetTankAiming) (Variables|Default|GetTankBarrel) (Variables|Default|GetTankTurret))
  (Class|TankMovementComponent|Initialise (Variables|Default|GetTankMovement) (Variables|Default|GetTankTracks_Left) (Variables|Default|GetTankTrack_Right))
  (CallFunction|InitialiseHealthBar))

(event Input|ActionEvents|InputActionSwitchCamera
  (params (Key :type Key%20Structure))
  ;[1 1 1] Camera Switch
  (:Released
    (Components|Activation|ToggleActive (Variables|Default|Get3rdPersonCamera))))

(event Input|AxisEvents|InputAxisAimAzimuth
  (params (AxisValue :type Float%20%28single-precision%29))
  ;[1 1 1] Camera Input Binding
  (Transformation|AddLocalRotation (Variables|Default|GetAzimuthGimbal) (Math|Rotator|MakeRotator 0.0 0.0 (* AxisValue (Utilities|Time|GetWorldDeltaSeconds) 1e+02)) false false))

(event Input|AxisEvents|InputAxisForwardMovement
  (params (AxisValue :type Float%20%28single-precision%29))
  ;[1 1 1] Move Input Binding
  (Class|TankMovementComponent|IntendMoveForward (Variables|Default|GetTankMovement) AxisValue))

(event Input|AxisEvents|InputAxisBackwardMovement
  (params (AxisValue :type Float%20%28single-precision%29))
  ;[1 1 1] Move Input Binding
  (Class|TankMovementComponent|IntendMoveBackward (Variables|Default|GetTankMovement) AxisValue))

(event Input|AxisEvents|InputAxisLeftMovement
  (params (AxisValue :type Float%20%28single-precision%29))
  ;[1 1 1] Move Input Binding
  (Class|TankMovementComponent|IntendMoveLeft (Variables|Default|GetTankMovement) AxisValue))

(event Input|AxisEvents|InputAxisAimAltitude
  (params (AxisValue :type Float%20%28single-precision%29))
  ;[1 1 1] Camera Input Binding
  (Transformation|AddLocalRotation (Variables|Default|GetSpringArm) (Math|Rotator|MakeRotator 0.0 (* AxisValue (Utilities|Time|GetWorldDeltaSeconds) 1e+02) 0.0) false false))

(event Input|AxisEvents|InputAxisLeftTrackThrottle
  (params (AxisValue :type Float%20%28single-precision%29))
  ;[1 1 1] Move Input Binding
  (Class|TankTracks|SetThrottle (Variables|Default|GetTankTracks_Left) AxisValue))

(event Input|AxisEvents|InputAxisRightTrackThrottle
  (params (AxisValue :type Float%20%28single-precision%29))
  ;[1 1 1] Move Input Binding
  (Class|TankTracks|SetThrottle (Variables|Default|GetTankTrack_Right) AxisValue))

(event Input|AxisEvents|InputAxisRightMovement
  (params (AxisValue :type Float%20%28single-precision%29))
  ;[1 1 1] Move Input Binding
  (Class|TankMovementComponent|IntendMoveRight (Variables|Default|GetTankMovement) AxisValue))

(event Input|MouseEvents|RightMouseButton
  (params (Key :type Key%20Structure))
  ;[1 1 1] Fire Input Binding
  (:Released
    (Class|TankAimingComponent|Fire (Variables|Default|GetTankAiming))))

(fn ConstructionScript)

(fn InitialiseHealthBar
  (bind _ashealth_bar (Utilities|Casting|CastToHealthBar (UserInterface|GetUserWidgetObject (Variables|Default|GetHealthBar))))
  (Variables|/Game/Blueprints/HealthBar.HealthBar_C|SetMyTank _ashealth_bar self))